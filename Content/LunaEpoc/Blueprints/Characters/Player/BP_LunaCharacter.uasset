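; Top-down player character for Luna that prototypes a line-of-sight vision cone, with GAS-backed health and stamina getters.
; On selected maps, a looping timer fans out head traces, draws the hits as triangles into a render target and updates a material parameter collection.
; Right mouse tweens cone shape, F tweens FOV, Tab toggles the effect.
; BeginPlay also sets up tilt-shift and a cursor-aimed light beam; Tick overrides the audio listener.
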(event Custom|UpdateLoSVisionSystem
  (bind _returnvalue (Game|GetPlayerController 0))
  (bind _returnvalue_2 (Transformation|GetActorLocation))
  (bind _lightbeam (Variables|Default|GetLightBeam))
  (bind _hitresult (Game|Player|GetHitResultUnderCursorbyChannel _returnvalue "TraceTypeQuery1" true))
  (bind _location (Collision|BreakHitResult _hitresult))
  (bind _returnvalue_3 (Math|Rotator|FindLookatRotation _returnvalue_2 _location))
  (bind _returnvalue_4 (Game|GetCurrentLevelName true))
  (if (Utilities|Enum|Equal(Enum) _returnvalue_4 "RadialLoS_v2")
    (Variables|LoSSystem|Tunables|SetNumberofTraces 360)
    (VisionConeSystemV2|LoSVisionSystem)
    (else
      (VisionConeSystemV2|LoSVisionSystem)
      (Transformation|SetActorLocation (Variables|Default|GetLightBeam) (Transformation|GetSocketLocation (Variables|Character|GetMesh) "head") false false)
      (Transformation|SetActorRotation _lightbeam (Math|Rotator|MakeRotator (.roll (Transformation|GetActorRotation _lightbeam)) (.pitch _returnvalue_3) (.yaw _returnvalue_3))))))

(event EventBeginPlay
  (Utilities|FlowControl|Sequence
    (:then_0
      (if (Variables|CameraVariables|GetUse%20Tilt%20Shift%20Effect)
        (bind _returnvalue (Game|AddComponentbyClass "/Script/Engine.PostProcessComponent" false))
        (Variables|Default|SetTiltShift_PP _returnvalue)
        (Utilities|Struct|SetmembersinPostProcessSettings (Variables|/Script/Engine.PostProcessComponent|GetSettings _returnvalue) (Variables|CameraVariables|GetCamera%20Aperture%20F-Stop) 144.0 (Variables|/Script/Engine.SpringArmComponent|GetTargetArmLength (Variables|Default|GetCameraBoom)))
        (bind _outactors (Actor|GetAllActorsOfClass "/Script/Engine.PostProcessVolume"))
        (bind _output_get (Variables|Components|SetPostProcessVolume (Utilities|Array|Get(acopy) _outactors)))
        (Variables|/Script/Engine.PostProcessVolume|SetBlendWeight _output_get 1.0)
        (bind _returnvalue_2 (Game|SpawnActorfromClass "/Game/LunaEpoc/Prototypes/Flashlight_Proto/Chracter_Light/LightBeam.LightBeam_C" (Math|Transform|MakeTransform (Transformation|GetSocketLocation (Variables|Character|GetMesh) "head") "0, 0, 0" "1.000000,1.000000,1.000000") "Undefined" "MultiplyWithRoot" 0 0))
        (bind _output_get_2 (Variables|Default|SetLightBeam _returnvalue_2))
        (Transformation|AttachActorToActor _output_get_2 self "head" "SnapToTarget" "SnapToTarget" "KeepRelative" true)))
    (:then_1
      (if (Variables|LoSSystem|GetActivateLoSProto)
        ;[1 1 1] Ensuring this Proto isn't interfering with other people's work
        (bind _returnvalue_3 (Game|GetCurrentLevelName true))
        (if (Math|Boolean|ORBoolean (Utilities|Enum|Equal(Enum) _returnvalue_3 "Main_Gameplay_Map") (Utilities|Enum|Equal(Enum) _returnvalue_3 "RadialLoS_v2") (Utilities|Enum|Equal(Enum) _returnvalue_3 "The_Massif"))
          (bind _returnvalue_4 (Utilities|Time|SetTimerbyEvent (delegate Custom|UpdateLoSVisionSystem) 0.01 true))
          (Variables|LoSSystem|SetLoSVisionSystemTimer _returnvalue_4))))
    (:then_2
      ;[1 1 1] Temp UI
      (UserInterface|CreateWidget "/Game/LunaEpoc/Blueprints/Widgets/WBP_HealthBar.WBP_HealthBar_C" (Game|GetPlayerController 0)))))

(event EventTick
  (params (DeltaSeconds :type Float%20%28single-precision%29))
  ;[1 0.1297 0.8247] Audio: Set Spatial Audio Listener
  (Class|PlayerController|SetAudioListenerOverride (Game|GetPlayerController 0) 0 (Transformation|GetWorldLocation (Variables|Character|GetMesh)) (Camera|GetCameraRotation (Game|GetPlayerCameraManager 0))))

(event Input|KeyboardEvents|F
  (params (Key :type Key%20Structure :default "None"))
  ;[1 1 1] Field of View Tests
  (:Pressed
    (Utilities|FlowControl|FlipFlop
      (:A
        (bind _newfov (Timeline|Transition%20FOV PlayFromStart)
          (:Update
            (Camera|SetFieldOfView (Variables|Default|GetTopDownCameraComponent) _newfov)
            (Class|AkGameplayStatics|SetRTPCValue "/Game/LunaEpoc/Audio/GameParameters/Default_Work_Unit/AKR_Camera_FOV.AKR_Camera_FOV" (Math|Float|MapRangeClamped _newfov 25.0 15.0 0.0 1e+02))
            (Development|PrintString (Utilities|String|ToString(Float) (Math|Float|MapRangeClamped _newfov 25.0 15.0 0.0 1e+02)) true true "(R=0.000000,G=0.660000,B=1.000000,A=1.000000)" 2.0 "Noewdfghdne"))))
      (:B
        (Timeline|Transition%20FOV Reverse)))))

(event Input|MouseEvents|RightMouseButton
  (params (Key :type Key%20Structure :default "None"))
  ;[1 1 1] Vision Cone Changing Size when Aiming Weapon Tests
  (:Pressed
    (Utilities|FlowControl|Sequence
      (:then_0
        (bind _interpolate_sightline_dpt (Timeline|Aim%20Weapon Play) ; Changes Degrees Per Trace of Vision Cone
          (:Update
            (Variables|LoSSystem|Tunables|SetDegreesPerTrace _interpolate_sightline_dpt))))
      (:then_1
        (bind _extend_range (Timeline|Vision%20Cone%20Range%20Transition Play) ; Changes Range of the Vision Cone when aiming
          (:Update
            (Variables|LoSSystem|Tunables|SetVisionConeLength _extend_range))))))
  (:Released
    (Utilities|FlowControl|Sequence
      (:then_0
        (Timeline|Aim%20Weapon Reverse))
      (:then_1
        (Timeline|Vision%20Cone%20Range%20Transition Reverse)))))

(event Input|KeyboardEvents|R
  (params (Key :type Key%20Structure :default "None"))
  ;[1 1 1] Top Down Camera Transition
)

(event Input|KeyboardEvents|Tab
  (params (Key :type Key%20Structure :default "None"))
  (bind _losvisionsystemtimer (Variables|LoSSystem|GetLoSVisionSystemTimer))
  (:Pressed
    (Utilities|FlowControl|FlipFlop
      (:A
        (Variables|/Script/Engine.PostProcessVolume|SetBlendWeight (Variables|Components|GetPostProcessVolume) 0.0)
        (Variables|LoSSystem|SetActivateLoSProto false)
        (Utilities|Time|PauseTimerbyHandle _losvisionsystemtimer))
      (:B
        (Variables|/Script/Engine.PostProcessVolume|SetBlendWeight (Variables|Components|GetPostProcessVolume) 1.0)
        (Variables|LoSSystem|SetActivateLoSProto true)
        (Utilities|Time|UnpauseTimerbyHandle _losvisionsystemtimer)))))

(fn ConstructionScript
  ;[1 1 1] Store starting camera boom length
  (Variables|CameraVariables|SetStartingCameraBoomLength (Variables|/Script/Engine.SpringArmComponent|GetTargetArmLength (Variables|Default|GetCameraBoom))))

(fn LoSVisionSystem
  (bind _losrendertarget (Variables|LoSSystem|GetLoSRenderTarget))
  (Utilities|FlowControl|Sequence
    (:then_0
      (Rendering|Material|SetVectorParameterValue "/Game/LunaEpoc/Assets/Materials/LoS_Material_Prototypes/LoS_Version_2/PlayerPosition.PlayerPosition" "PlayerPosition" (Math|Conversions|ToLinearColor(Vector) (Transformation|GetActorLocation)) :!class /Script/Engine.KismetMaterialLibrary)
      (Rendering|Material|SetScalarParameterValue "/Game/LunaEpoc/Assets/Materials/LoS_Material_Prototypes/LoS_Version_2/PlayerPosition.PlayerPosition" "VisionConeScale" (Variables|LoSSystem|Tunables|GetVisionConeLength) :!class /Script/Engine.KismetMaterialLibrary)
      (Rendering|Material|SetVectorParameterValue "/Game/LunaEpoc/Assets/Materials/LoS_Material_Prototypes/LoS_Version_2/PlayerPosition.PlayerPosition" "PlayerForwardVector" (Math|Conversions|ToLinearColor(Vector) (Transformation|GetActorForwardVector)) :!class /Script/Engine.KismetMaterialLibrary)
      (Rendering|Material|SetVectorParameterValue "/Game/LunaEpoc/Assets/Materials/LoS_Material_Prototypes/LoS_Version_2/PlayerPosition.PlayerPosition" "PlayerRightVector" (Math|Conversions|ToLinearColor(Vector) (Transformation|GetActorRightVector)) :!class /Script/Engine.KismetMaterialLibrary)
      (Rendering|Material|SetVectorParameterValue "/Game/LunaEpoc/Assets/Materials/LoS_Material_Prototypes/LoS_Version_2/PlayerPosition.PlayerPosition" "PlayerUpVector" (Math|Conversions|ToLinearColor(Vector) (Transformation|GetActorUpVector)) :!class /Script/Engine.KismetMaterialLibrary))
    (:then_1
      (VisionConeSystemV2|CreateCone))
    (:then_2
      (VisionConeSystemV2|PrepareTrianglesforCanvas))
    (:then_3
      (Rendering|ClearRenderTarget2D _losrendertarget)
      (bind (_canvas _size _context) (Rendering|BeginDrawCanvastoRenderTarget _losrendertarget))
      (Class|Canvas|DrawTriangle _canvas 0 (Variables|LoSSystem|GetCanvasTriangles))
      (Rendering|EndDrawCanvastoRenderTarget _context))))

(fn CreateCone
  (bind _traceresults (Variables|LoSSystem|GetTraceResults))
  (bind _mesh (Variables|Character|GetMesh))
  (bind _returnvalue (Transformation|GetSocketLocation _mesh "head"))
  (Utilities|Array|Clear (Variables|LoSSystem|GetTraceResults))
  (for _index (range 0 (Variables|LoSSystem|Tunables|GetNumberofTraces))
    (bind (_outhit _returnvalue_2) (Collision|LineTraceByChannel _returnvalue (+ (* (Math|Vector|RotateVector (Math|Vector|RotateVector (Transformation|GetActorForwardVector) (Math|Rotator|MakeRotator 0.0 0.0 (/ (* (Variables|LoSSystem|Tunables|GetNumberofTraces) (Variables|LoSSystem|Tunables|GetDegreesPerTrace)) -2.0))) (Math|Rotator|MakeRotator 0.0 0.0 (* _index (Variables|LoSSystem|Tunables|GetDegreesPerTrace)))) (Variables|LoSSystem|Tunables|GetVisionConeLength)) _returnvalue) "TraceTypeQuery3" false 0 "None"))
    (if _returnvalue_2
      (Utilities|Array|Add _traceresults (+ (* (Math|Vector|RotateVector (Math|Vector|RotateVector (Transformation|GetActorForwardVector) (Math|Rotator|MakeRotator 0.0 0.0 (/ (* (Variables|LoSSystem|Tunables|GetNumberofTraces) (Variables|LoSSystem|Tunables|GetDegreesPerTrace)) -2.0))) (Math|Rotator|MakeRotator 0.0 0.0 (* _index (Variables|LoSSystem|Tunables|GetDegreesPerTrace)))) (Variables|LoSSystem|Tunables|GetLineTraceExtension)) (.location _outhit)))
      (else
        (Utilities|Array|Add _traceresults (+ (* (Math|Vector|RotateVector (Math|Vector|RotateVector (Transformation|GetActorForwardVector) (Math|Rotator|MakeRotator 0.0 0.0 (/ (* (Variables|LoSSystem|Tunables|GetNumberofTraces) (Variables|LoSSystem|Tunables|GetDegreesPerTrace)) -2.0))) (Math|Rotator|MakeRotator 0.0 0.0 (* _index (Variables|LoSSystem|Tunables|GetDegreesPerTrace)))) (Variables|LoSSystem|Tunables|GetLineTraceExtension)) (+ (* (Math|Vector|RotateVector (Math|Vector|RotateVector (Transformation|GetActorForwardVector) (Math|Rotator|MakeRotator 0.0 0.0 (/ (* (Variables|LoSSystem|Tunables|GetNumberofTraces) (Variables|LoSSystem|Tunables|GetDegreesPerTrace)) -2.0))) (Math|Rotator|MakeRotator 0.0 0.0 (* _index (Variables|LoSSystem|Tunables|GetDegreesPerTrace)))) (Variables|LoSSystem|Tunables|GetVisionConeLength)) _returnvalue)))))))

(fn PrepareTrianglesforCanvas
  (bind _returnvalue (Transformation|GetActorLocation))
  (bind _traceresults (Variables|LoSSystem|GetTraceResults))
  (bind _offset (Variables|LoSSystem|Tunables|GetOffset))
  (bind _returnvalue_2 (Math|Vector|MakeVector _offset _offset 0.0))
  (Utilities|Array|Clear (Variables|LoSSystem|GetCanvasTriangles))
  (for _index (range 0 (- (Utilities|Array|Length (Variables|LoSSystem|GetTraceResults)) 2))
    (Utilities|Array|Add (Variables|LoSSystem|GetCanvasTriangles) (Utilities|Struct|MakeCanvasUVTri (Math|Conversions|ToVector2D(Vector) _returnvalue_2) "(X=0.000000,Y=0.000000)" "(R=1.000000,G=1.000000,B=1.000000,A=0.000000)" (Math|Conversions|ToVector2D(Vector) (+ (- (Utilities|Array|Get(acopy) _traceresults _index) _returnvalue) _returnvalue_2)) "(X=0.000000,Y=0.000000)" "(R=1.000000,G=1.000000,B=1.000000,A=0.000000)" (Math|Conversions|ToVector2D(Vector) (+ (- (Utilities|Array|Get(acopy) _traceresults (+ _index 1)) _returnvalue) _returnvalue_2)) "(X=0.000000,Y=0.000000)" "(R=1.000000,G=1.000000,B=1.000000,A=0.000000)"))))

(fn GetHealth
  (return (.ReturnValue (Ability|Attribute|GetFloatAttributefromAbilitySystemComponent (Ability|GetAbilitySystemComponent 0) "(AttributeName=\"Health\",Attribute=/Script/LunaEpoc.LunaAttributeSet:Health,AttributeOwner=\"/Script/CoreUObject.Class'/Script/LunaEpoc.LunaAttributeSet'\")"))))

(fn GetStamina
  (return (.ReturnValue (Ability|Attribute|GetFloatAttributefromAbilitySystemComponent (Ability|GetAbilitySystemComponent 0) "(AttributeName=\"Stamina\",Attribute=/Script/LunaEpoc.LunaAttributeSet:Stamina,AttributeOwner=\"/Script/CoreUObject.Class'/Script/LunaEpoc.LunaAttributeSet'\")"))))