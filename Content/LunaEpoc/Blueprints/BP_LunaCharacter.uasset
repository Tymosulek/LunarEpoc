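; BP_LunaCharacter is a character Blueprint using the Gameplay Ability System, with a punch ability and an optional tilt-shift camera look.
; On BeginPlay it caches walk speed and, only if tilt-shift is enabled, adds a depth-of-field post process focused at camera boom length plus a placeholder HUD.
; The punch input activates GA_Punch through the ability system component.
; Health and Stamina getters read float attributes from that component.
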(event Input|EnhancedActionEvents|EnhancedInputActionIA_Punch
  (params (ActionValue :type Boolean) (ElapsedSeconds :type Float%20%28double-precision%29) (TriggeredSeconds :type Float%20%28double-precision%29) (InputAction :type Input%20Action%20Object%20Reference :default "/Game/LunaEpoc/Input/Actions/IA_Punch.IA_Punch"))
  (Abilities|TryActivateAbilitybyClass (Variables|Default|GetAbilitySystemComponent) "/Game/LunaEpoc/Abilities/GA_Punch.GA_Punch_C" true))

(event EventBeginPlay
  (Variables|CharacterMovement|SetDefault%20Walk%20Speed%20%28old%29 (Variables|/Script/Engine.CharacterMovementComponent|GetMaxWalkSpeed (Variables|Character|GetCharacterMovement)))
  (if (Variables|CameraVariables|GetUse%20Tilt%20Shift%20Effect)
    (bind _returnvalue (Game|AddComponentbyClass "/Script/Engine.PostProcessComponent" false))
    (Utilities|Struct|SetmembersinPostProcessSettings (Variables|/Script/Engine.PostProcessComponent|GetSettings _returnvalue) (Variables|CameraVariables|GetCamera%20Aperture%20F-Stop) 144.0 (Variables|/Script/Engine.SpringArmComponent|GetTargetArmLength (Variables|Default|GetCameraBoom)))
    ;[1 1 1] Placeholder HUD
    (bind _returnvalue_2 (UserInterface|CreateWidget "/Game/LunaEpoc/UI/Widgets/WBP_HUD.WBP_HUD_C" (Game|GetPlayerController 0)))
    (UserInterface|Viewport|AddtoViewport _returnvalue_2 0)))

(fn ConstructionScript)

(fn GetHealth
  (return (.ReturnValue (Ability|Attribute|GetFloatAttributefromAbilitySystemComponent (Ability|GetAbilitySystemComponent 0) "(AttributeName=\"Health\",Attribute=/Script/LunaEpoc.LunaAttributeSet:Health,AttributeOwner=\"/Script/CoreUObject.Class'/Script/LunaEpoc.LunaAttributeSet'\")"))))

(fn GetStamina
  (return (.ReturnValue (Ability|Attribute|GetFloatAttributefromAbilitySystemComponent (Ability|GetAbilitySystemComponent 0) "(AttributeName=\"Stamina\",Attribute=/Script/LunaEpoc.LunaAttributeSet:Stamina,AttributeOwner=\"/Script/CoreUObject.Class'/Script/LunaEpoc.LunaAttributeSet'\")"))))