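; Room manager actor that ties a room's doorways to a camera perspective: isometric, top-down or side-scrolling.
; On BeginPlay it binds to each doorway's player-entering event, then broadcasts OnRoomEntered with its perspective, plus a debug print.
; The construction script runs ChangeRoomState, which hides in game the occludable objects listed for that perspective and unhides the other two lists.
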(event Custom|SignalCameraManager
  (Default|CallOnRoomEntered (Variables|CameraPerspective|GetPlayerCameraPerspective))
  (Development|PrintString "bind"))

(event EventBeginPlay
  (for _array_element (Variables|Default|GetDoorways)
    (EventDispatchers|BindEventtoPlayerEnteringRoom _array_element (delegate Custom|SignalCameraManager))))

(event Collision|EventActorBeginOverlap
  (params (OtherActor :type Actor%20Object%20Reference)))

(event EventTick
  (params (DeltaSeconds :type Float%20%28single-precision%29)))

(fn ConstructionScript
  (CallFunction|ChangeRoomState))

(fn ChangeRoomState
  (switch Utilities|FlowControl|Switch|SwitchonPlayer_Camera_Perspectives (Variables|CameraPerspective|GetPlayerCameraPerspective)
    (:NewEnumerator0
      (for _array_element (Variables|CameraPerspective|Occludables|GetTopDown_Occludable_Objects)
        (Rendering|SetActorHiddenInGame _array_element false))
      (for _array_element_2 (Variables|CameraPerspective|Occludables|GetSideScroll_Occludable_Objects)
        (Rendering|SetActorHiddenInGame _array_element_2 false))
      (for _array_element_3 (Variables|CameraPerspective|Occludables|GetIso_Occludable_Objects)
        (Rendering|SetActorHiddenInGame _array_element_3 true)))
    (:NewEnumerator1
      (for _array_element_4 (Variables|CameraPerspective|Occludables|GetIso_Occludable_Objects)
        (Rendering|SetActorHiddenInGame _array_element_4 false))
      (for _array_element_5 (Variables|CameraPerspective|Occludables|GetSideScroll_Occludable_Objects)
        (Rendering|SetActorHiddenInGame _array_element_5 false))
      (for _array_element_6 (Variables|CameraPerspective|Occludables|GetTopDown_Occludable_Objects)
        (Rendering|SetActorHiddenInGame _array_element_6 true)))
    (:NewEnumerator2
      (for _array_element_7 (Variables|CameraPerspective|Occludables|GetIso_Occludable_Objects)
        (Rendering|SetActorHiddenInGame _array_element_7 false))
      (for _array_element_8 (Variables|CameraPerspective|Occludables|GetTopDown_Occludable_Objects)
        (Rendering|SetActorHiddenInGame _array_element_8 false))
      (for _array_element_9 (Variables|CameraPerspective|Occludables|GetSideScroll_Occludable_Objects)
        (Rendering|SetActorHiddenInGame _array_element_9 true)))))