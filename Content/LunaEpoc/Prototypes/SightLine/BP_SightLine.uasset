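; Prototype line-of-sight actor that follows the first actor of ClassToFollow and maps what it can see.
; Each tick it fires a fan of visibility traces, stretching one instanced mesh per ray to the hit distance and recording hit components.
; An orthographic scene capture and MPC_Sightline parameters appear to turn that shape into a material mask.
; Hit components get their Mask material parameter zeroed only at construction.
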(event EventBeginPlay
  ;[1 1 1] Once prototype is complete replace this with just attaching the BP_SightLine object as a component onto the player character. Doing it this way so it's only visible in the map the BP_Sightline is placed in (Mikes test map) so it doesnt get in the way of others' work.
  (bind _outactors (Actor|GetAllActorsOfClass (Variables|Constants|GetClassToFollow)))
  (Variables|Constants|SetActorToFollow (Utilities|Array|Get(acopy) _outactors)))

(event Collision|EventActorBeginOverlap
  (params (OtherActor :type Actor%20Object%20Reference)))

(event EventTick
  (params (DeltaSeconds :type Float%20%28single-precision%29))
  ;[1 1 1] Once prototype is complete replace this with just attaching the BP_SightLine object as a component onto the player character. Doing it this way so it's only visible in the map the BP_Sightline is placed in (Mikes test map) so it doesnt get in the way of others' work.
  (bind _actortofollow (Variables|Constants|GetActorToFollow)
    (:then
      (Transformation|SetActorLocation (Transformation|GetActorLocation _actortofollow) false false)
      (Transformation|SetActorRotation (Math|Rotator|MakeRotator (.roll (Transformation|GetActorRotation _actortofollow)) (.pitch (Transformation|GetActorRotation _actortofollow)) (.yaw (Transformation|GetActorRotation _actortofollow))))
      (CallFunction|SightTrace)
      (Rendering|Material|SetVectorParameterValue "/Game/LunaEpoc/Assets/Materials/LoS_Material_Prototypes/LoS_Version_1/MPC_Sightline.MPC_Sightline" "SightLineActorLocation" (Math|Conversions|ToLinearColor(Vector) (Transformation|GetActorLocation)) :!class /Script/Engine.KismetMaterialLibrary))
    (:else)))

(fn ConstructionScript
  (CallFunction|InitializeISM))

(fn SightTrace
  (bind _returnvalue (Transformation|GetActorLocation))
  (bind _tracecount (Variables|Constants|GetTraceCount))
  (Utilities|Array|Clear (Variables|Default|GetActorWithinView))
  (Utilities|Array|Clear (Variables|Default|GetObjectsWithinView))
  (for _index (range 0 (- (Variables|Constants|GetTraceCount) 1))
    (bind _output_get (Variables|Constants|SetCurrentTraceStep _index))
    (bind (_outhit _returnvalue_2) (Collision|LineTraceByChannel _returnvalue (+ _returnvalue (* (Math|Vector|RotateVector (Math|Vector|RotateVector (Transformation|GetActorForwardVector) (Math|Rotator|MakeRotator 0.0 0.0 (/ (* (Variables|Constants|GetTraceCount) (Variables|Constants|GetDegrees%20Per%20Trace)) -2.0))) (Math|Rotator|MakeRotator 0.0 0.0 (* _output_get (Variables|Constants|GetDegrees%20Per%20Trace)))) (Variables|Tunables|GetCheckRange))) "TraceTypeQuery1" false 0 "None" false "(R=1.000000,G=0.000000,B=0.000000,A=1.000000)" "(R=0.000000,G=1.000000,B=0.000000,A=1.000000)" 0.1))
    (Components|InstancedStaticMesh|UpdateInstanceTransform (Variables|Default|GetInstancedStaticMesh) (Variables|Constants|GetCurrentTraceStep) (Math|Transform|MakeTransform (Math|Vector|SelectVector (Math|Vector|MakeVector 0.0 0.0 (Variables|Tunables|GetISM_HeightOffset)) "0, 0, 0" (Variables|Default|GetOffsetByHeight)) (Math|Rotator|FindLookatRotation (.TraceStart (Collision|BreakHitResult _outhit)) (.TraceEnd (Collision|BreakHitResult _outhit))) (Math|Vector|MakeVector (* (Math|Vector|VectorLength (- (Math|Vector|SelectVector (.Location (Collision|BreakHitResult _outhit)) (.TraceEnd (Collision|BreakHitResult _outhit)) _returnvalue_2) (.TraceStart (Collision|BreakHitResult _outhit)))) (Variables|Tunables|GetTraceHitOffset)) (* (/ _tracecount _tracecount) (* (Math|Vector|VectorLength (- (Math|Vector|SelectVector (.Location (Collision|BreakHitResult _outhit)) (.TraceEnd (Collision|BreakHitResult _outhit)) _returnvalue_2) (.TraceStart (Collision|BreakHitResult _outhit)))) (Variables|Tunables|GetTraceHitOffset))) (* (Math|Vector|VectorLength (- (Math|Vector|SelectVector (.Location (Collision|BreakHitResult _outhit)) (.TraceEnd (Collision|BreakHitResult _outhit)) _returnvalue_2) (.TraceStart (Collision|BreakHitResult _outhit)))) (Variables|Tunables|GetTraceHitOffset)))) false true true)
    (if _returnvalue_2
      (Utilities|Array|Add (Variables|Default|GetObjectsWithinView) (.HitComponent (Collision|BreakHitResult _outhit)))
      (Development|PrintString (Utilities|String|Append "ADDING " (Utilities|GetDisplayName (.HitComponent (Collision|BreakHitResult _outhit))) "  TO ARRAY:") false false "(R=0.120583,G=1.000000,B=0.000000,A=1.000000)" 0.01)
      (Development|PrintString (Utilities|String|ToString(Integer) (Utilities|Array|Length (Variables|Default|GetObjectsWithinView))) false false "(R=0.120583,G=1.000000,B=0.000000,A=1.000000)" 0.01))))

(fn InitializeISM
  (bind _scenecapturecomponent2d (Variables|Default|GetSceneCaptureComponent2D))
  (Components|InstancedStaticMesh|ClearInstances (Variables|Default|GetInstancedStaticMesh))
  (for _index (range 0 (- (Variables|Constants|GetTraceCount) 1))
    (Components|InstancedStaticMesh|AddInstance (Variables|Default|GetInstancedStaticMesh) (Math|Transform|MakeTransform "0, 0, 0") false))
  (CallFunction|SightTrace)
  (CallFunction|SetViewableObjectMaterial)
  (Variables|/Script/Engine.SceneCaptureComponent2D|SetOrthoWidth _scenecapturecomponent2d (Variables|Tunables|GetCheckRange))
  (Transformation|SetRelativeTransform _scenecapturecomponent2d (Math|Transform|MakeTransform (Math|Vector|MakeVector 0.0 0.0 (- (Variables|Tunables|GetISM_HeightOffset) 1.0)) "90.000000,0.000000,0.000000" "1.000000,-1.000000,-1.000000") false false)
  (Rendering|Material|SetScalarParameterValue "/Game/LunaEpoc/Assets/Materials/LoS_Material_Prototypes/LoS_Version_1/MPC_Sightline.MPC_Sightline" "SightLineMaskHeight" (+ (.z (Transformation|GetActorLocation)) (Variables|Tunables|GetISM_HeightOffset) -5e+02) :!class /Script/Engine.KismetMaterialLibrary)
  (Rendering|Material|SetScalarParameterValue "/Game/LunaEpoc/Assets/Materials/LoS_Material_Prototypes/LoS_Version_1/MPC_Sightline.MPC_Sightline" "SightLineTexScale" (Variables|Tunables|GetCheckRange) :!class /Script/Engine.KismetMaterialLibrary)
  (Rendering|Material|SetVectorParameterValue "/Game/LunaEpoc/Assets/Materials/LoS_Material_Prototypes/LoS_Version_1/MPC_Sightline.MPC_Sightline" "SightLineActorLocation" (Math|Conversions|ToLinearColor(Vector) (Transformation|GetActorLocation)) :!class /Script/Engine.KismetMaterialLibrary))

(fn SetViewableObjectMaterial
  (for _array_element (Variables|Default|GetObjectsWithinView)
    (bind _returnvalue (Rendering|Material|CreateDynamicMaterialInstance _array_element 0 (Rendering|Material|GetMaterial _array_element 0) "None" :!class /Script/Engine.PrimitiveComponent))
    (Rendering|Material|SetScalarParameterValue _returnvalue "Mask" 0.0 :!class /Script/Engine.MaterialInstanceDynamic)))