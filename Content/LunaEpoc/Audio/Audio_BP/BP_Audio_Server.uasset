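; Ambient audio actor that plays a looping server tower sound while an actor is inside its Box trigger.
; Begin and end overlap post Wwise play and stop events, gated by two DoOnce nodes that re-arm each other to prevent repeats.
; From BeginPlay, a self-recalling delayed MoveAudio event keeps the Ak component and Arrow at the Spline point closest to the player character, so the emitter follows along the spline.
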(event OnComponentBeginOverlap(Box)
  (params (OverlappedComponent :type Primitive%20Component%20Object%20Reference) (OtherActor :type Actor%20Object%20Reference) (OtherComp :type Primitive%20Component%20Object%20Reference) (OtherBodyIndex :type Integer) (bFromSweep :type Boolean) (SweepResult :type Hit%20Result%20Structure%20%28by%20ref%29))
  (Utilities|FlowControl|DoOnce false
    (:Completed
      (Class|AkGameObject|PostAkEvent (Variables|Default|GetAk) "/Game/LunaEpoc/Audio/Events/Default_Work_Unit/Ambience/Environments/AKE_PlayAmb_ServerTower_Lp.AKE_PlayAmb_ServerTower_Lp")
      (Utilities|FlowControl|DoOnce false) ; enters at Reset
    )))

(event OnComponentEndOverlap(Box)
  (params (OverlappedComponent :type Primitive%20Component%20Object%20Reference) (OtherActor :type Actor%20Object%20Reference) (OtherComp :type Primitive%20Component%20Object%20Reference) (OtherBodyIndex :type Integer))
  (Utilities|FlowControl|DoOnce false
    (:Completed
      (Class|AkGameObject|PostAkEvent (Variables|Default|GetAk) "/Game/LunaEpoc/Audio/Events/Default_Work_Unit/Ambience/Environments/AKE_StopAmb_ServerTower_Lp.AKE_StopAmb_ServerTower_Lp")
      (Utilities|FlowControl|DoOnce false) ; enters at Reset
    )))

(event Custom|Move%20Audio
  (bind _character_ref (Variables|Default|GetCharacter%20REF))
  (bind _spline (Variables|Default|GetSpline))
  (bind _returnvalue (Transformation|GetActorLocation _character_ref))
  (bind _returnvalue_2 (Spline|FindLocationClosesttoWorldLocation _spline _returnvalue "World"))
  ;[0.9301 0.1878 0.9216 0.502] Sets location of Audio object to follow Character REF along Spline.
  (Transformation|SetWorldLocation (Variables|Default|GetArrow) (Math|Vector|MakeVector (.x _returnvalue_2) (.y _returnvalue_2) (.z _returnvalue_2)) false false)
  (Utilities|FlowControl|Delay 0.05)
  (CallFunction|MoveAudio))

(event EventBeginPlay
  ;[0.9301 0.1878 0.9216 0.502] Creates 'Character REF' from player, trigger custom 'Move Audio' Event
  (bind _asluna_character (Utilities|Casting|CastToLunaCharacter (Game|GetPlayerCharacter 0)))
  (Variables|Default|SetCharacter%20REF _asluna_character)
  (CallFunction|MoveAudio))

(fn ConstructionScript)