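; Audio timer actor that alternates Day and Night countdowns to drive Wwise music and room-tone ambience.
; TimerToggle uses a FlipFlop to reset the phase's duration and RTPC, set the music State and ambience Switch, and start a one-second looping timer.
; CountdownDay and CountdownNight send remaining time as a 0-100 interpolated RTPC.
; At zero, each posts an end sound, clears its timer and calls TimerToggle again.
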(event Custom|Timer_Day
  ;[0.702 0.03922 0.2392] Countdown Logic
  ;;[0 0.9608 1] Resets RTPCs/States, Triggers Countdown Sequence
  ;;;[1 0.4706 0] Day Countdown ☀️
  (CallFunction|CountdownDay))

(event Custom|TimerToggle
  ;[0.702 0.03922 0.2392] Countdown Logic
  (Utilities|FlowControl|FlipFlop ; Toggles between Day and Night Timers
    (:A
      ;;[0 0.9608 1] Resets RTPCs/States, Triggers Countdown Sequence
      ;;;[1 0.4706 0] Day Countdown ☀️
      (Development|PrintString "DAY" true true "(R=0.000000,G=0.710351,B=1.000000,A=1.000000)" 2.0 "erfefrfer")
      (Variables|Default|SetCountdown_Day%28Seconds%29 (Variables|Default|GetCountdown_Day_Duration)) ; Sets Countdown Duration for Day
      (Class|AkGameplayStatics|ResetRTPCValue "/Game/LunaEpoc/Audio/GameParameters/AKR_Desync_TimeRemaining_Day.AKR_Desync_TimeRemaining_Day" 0 self "None") ; Resets RTPC for Day
      (Class|AkGameplayStatics|SetState "/Game/LunaEpoc/Audio/States/AKST_Desync-Desync_Day.AKST_Desync-Desync_Day") ; Uses Day State to play Music
      (Class|AkGameplayStatics|SetSwitch "/Game/LunaEpoc/Audio/Switches/AKSW_DayNight/AKSW_DayNight-Day.AKSW_DayNight-Day" self) ; Switches  Ambience to Day
      (bind _returnvalue (Utilities|Time|SetTimerbyEvent (delegate Custom|Timer_Day) 1.0 true false 1.0))
      (Variables|Default|SetDesync_Timer_Day _returnvalue))
    (:B
      ;;;[0.1059 0 1] Night Countdown 🌕
      (Development|PrintString "NIGHT" true true "(R=1.000000,G=0.000000,B=0.070588,A=1.000000)" 2.0 "reefrefr")
      (Variables|Default|SetCountdown_Night%28Seconds%29 (Variables|Default|GetCountdown_Night_Duration)) ; Sets Countdown Duration for Night
      (Class|AkGameplayStatics|ResetRTPCValue "/Game/LunaEpoc/Audio/GameParameters/AKR_Desync_TimeRemaining_Night.AKR_Desync_TimeRemaining_Night" 0 self "None") ; Resets RTPC for Night
      (Class|AkGameplayStatics|SetState "/Game/LunaEpoc/Audio/States/AKST_Desync-Desync_Night.AKST_Desync-Desync_Night") ; Uses Night State to Stop Music
      (Class|AkGameplayStatics|SetSwitch "/Game/LunaEpoc/Audio/Switches/AKSW_DayNight/AKSW_DayNight-Night.AKSW_DayNight-Night" self) ; Switches Ambience to Night
      (bind _returnvalue_2 (Utilities|Time|SetTimerbyEvent (delegate Custom|Timer_Night) 1.0 true false 1.0))
      (Variables|Default|SetDesync_Timer_Night _returnvalue_2))))

(event Custom|Timer_Night
  ;[0.702 0.03922 0.2392] Countdown Logic
  ;;[0 0.9608 1] Resets RTPCs/States, Triggers Countdown Sequence
  ;;;[0.1059 0 1] Night Countdown 🌕
  (CallFunction|CountdownNight))

(event EventBeginPlay
  (bind _self self)
  ;[0.702 0.03922 0.2392] Countdown Logic
  (CallFunction|TimerToggle) ; Triggers Day countdown on launch
  (Class|AkGameplayStatics|PostEvent "/Game/LunaEpoc/Audio/Events/Default_Work_Unit/Ambience/Roomtone/AKE_PlayAmb_Roomtone.AKE_PlayAmb_Roomtone" _self) ; Plays Ambience Switch Container
  (Variables|Default|SetSwitch_Ref _self))

(fn ConstructionScript)

(fn CountdownDay
  (Utilities|FlowControl|Sequence
    (:then_0
      ;[1 0.4706 0] Subtracts 1 second from the countdown on each Event Call
      (bind _output_get (Variables|Default|SetCountdown_Day%28Seconds%29 (- (Variables|Default|GetCountdown_Day%28Seconds%29) 1.0)))
      (Development|PrintString (Utilities|String|ToString(Float) _output_get) true true "(R=0.000000,G=0.660000,B=1.000000,A=1.000000)" 2.0 "Nondgyulae"))
    (:then_1
      ;[1 0.4706 0] Clamps the countdown to 0-100, so it can be used as a percentage, updates RTPC
      (bind _output_get_2 (Variables|Default|SetCountdown_Day%28Percentage%29 (Math|Float|MapRangeClamped (Variables|Default|GetCountdown_Day%28Seconds%29) 0.0 (Variables|Default|GetCountdown_Day_Duration) 0.0 1e+02)))
      (Class|AkGameplayStatics|SetRTPCValue "/Game/LunaEpoc/Audio/GameParameters/AKR_Desync_TimeRemaining_Day.AKR_Desync_TimeRemaining_Day" _output_get_2 1000 self))
    (:then_2
      ;[1 0.4706 0] When Countdown reaches 0, trigger audio events, and clear timer
      (if (== (Variables|Default|GetCountdown_Day%28Seconds%29) 0.0)
        (Utilities|FlowControl|Sequence
          (:then_0
            (Class|AkGameplayStatics|PostEvent "/Game/LunaEpoc/Audio/Events/Default_Work_Unit/UI/Desync/AKE_PlayUI_DayCountdownEnd.AKE_PlayUI_DayCountdownEnd") ; Plays Countdown End
            (Class|AkGameplayStatics|SetSwitch "/Game/LunaEpoc/Audio/Switches/AKSW_DayNight/AKSW_DayNight-Night.AKSW_DayNight-Night" self))
          (:then_1
            (Utilities|Time|ClearandInvalidateTimerbyHandle (Variables|Default|GetDesync_Timer_Day))
            (CallFunction|TimerToggle)))))))

(fn CountdownNight
  (Utilities|FlowControl|Sequence
    (:then_0
      ;[0.1059 0 1] Subtracts 1 second from the countdown on each Event Call
      (bind _output_get (Variables|Default|SetCountdown_Night%28Seconds%29 (- (Variables|Default|GetCountdown_Night%28Seconds%29) 1.0)))
      (Development|PrintString (Utilities|String|ToString(Float) _output_get) true true "(R=1.000000,G=0.000000,B=0.070588,A=1.000000)" 2.0 "Nondgyulae"))
    (:then_1
      ;[0.1059 0 1] Clamps the countdown to 0-100, so it can be used as a percentage, updates RTPC
      (bind _output_get_2 (Variables|Default|SetCountdown_Night%28Percentage%29 (Math|Float|MapRangeClamped (Variables|Default|GetCountdown_Night%28Seconds%29) 0.0 (Variables|Default|GetCountdown_Night_Duration) 0.0 1e+02)))
      (Class|AkGameplayStatics|SetRTPCValue "/Game/LunaEpoc/Audio/GameParameters/AKR_Desync_TimeRemaining_Night.AKR_Desync_TimeRemaining_Night" _output_get_2 1000 self))
    (:then_2
      ;[0.1059 0 1] When Countdown reaches 0, trigger audio events, and clear timer
      (if (== (Variables|Default|GetCountdown_Night%28Percentage%29) 0.0)
        (Utilities|FlowControl|Sequence
          (:then_0
            (Class|AkGameplayStatics|PostEvent "/Game/LunaEpoc/Audio/Events/Default_Work_Unit/UI/Desync/AKE_PlayUI_NightCountdownEnd.AKE_PlayUI_NightCountdownEnd") ; Plays Countdown End
            (Class|AkGameplayStatics|SetSwitch "/Game/LunaEpoc/Audio/Switches/AKSW_DayNight/AKSW_DayNight-Night.AKSW_DayNight-Night" self))
          (:then_1
            (Utilities|Time|ClearandInvalidateTimerbyHandle (Variables|Default|GetDesync_Timer_Night))
            (CallFunction|TimerToggle)))))))