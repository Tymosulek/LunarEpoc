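; BP_Audio_WindSpline is a spline-based audio actor, named for wind, that keeps a Wwise sound source at the point on its path nearest the player.
; BeginPlay caches the BP_LunaCharacter and starts MoveAudio, which moves the AkGameObject and an Arrow to that closest spline point, raised slightly.
; MoveAudio re-calls itself through a zero-length Delay, updating every frame without Event Tick.
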(event Custom|MoveAudio
  (bind _character_reference (Variables|Default|GetCharacter%20Reference))
  (bind _spline (Variables|Default|GetSpline))
  (bind _returnvalue (Transformation|GetActorLocation _character_reference))
  (bind _returnvalue_2 (Spline|FindLocationClosesttoWorldLocation _spline _returnvalue "World"))
  (Transformation|SetWorldLocation (Variables|Default|GetArrow) (Math|Vector|MakeVector (.x _returnvalue_2) (.y _returnvalue_2) (+ (.z _returnvalue_2) 5e+01)) false false)
  (Utilities|FlowControl|Delay 0.0)
  (CallFunction|MoveAudio))

(event EventBeginPlay
  (bind _asbp_luna_character (Utilities|Casting|CastToBP_LunaCharacter (Game|GetPlayerCharacter 0)))
  (Variables|Default|SetCharacter%20Reference _asbp_luna_character)
  (CallFunction|MoveAudio))

(fn ConstructionScript)