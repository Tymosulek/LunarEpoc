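; Audio occlusion Blueprint that drives the Wwise AKR_Occlusion RTPC from world geometry between a sound source and the player.
; BeginPlay caches the first BP_Vent's location as the source.
; Each Tick multi-traces WorldStatic objects to the player, scaling hit count by OcclusionPercentage with one-second interpolation, or resetting when clear.
; It also stores player distance, unused here, and leaves debug traces and prints active.
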(event EventBeginPlay
  (bind _outactors (Actor|GetAllActorsOfClass "/Game/LunaEpoc/Assets/Props/BP_Vent.BP_Vent_C"))
  (bind _output_get (Variables|Default|SetSourceLocation (Transformation|GetActorLocation (Utilities|Array|Get(acopy) _outactors))))
  (Variables|Default|SetDistance (Math|Vector|VectorLength (- (stale EventTick _output_get) _output_get))))

(event EventTick
  (params (DeltaSeconds :type Float%20%28single-precision%29))
  (Utilities|FlowControl|Sequence
    (:then_0
      (bind _output_get (Variables|Default|SetPlayerLocation (Transformation|GetActorLocation (Game|GetPlayerCharacter 0))))
      (Variables|Default|SetDistance (Math|Vector|VectorLength (- _output_get (stale EventBeginPlay _output_get)))))
    (:then_1
      (bind (_outhits _returnvalue) (Class|KismetSystemLibrary|LineTraceMultiforObjects (Variables|Default|GetSourceLocation) (Variables|Default|GetPlayerLocation) (Utilities|Array|MakeArray "ObjectTypeQuery1") false 0 "ForDuration" true "(R=1.000000,G=0.000000,B=0.000000,A=1.000000)" "(R=0.000000,G=1.000000,B=0.000000,A=1.000000)" 0.1))
      (if _returnvalue
        (Development|PrintString "IS_Occluded" true true "(R=0.000000,G=0.660000,B=1.000000,A=1.000000)" 2.0 "dfsd")
        (Class|AkGameplayStatics|SetRTPCValue "/Game/WwiseAudio/Game_Parameters/Default_Work_Unit/Ambience/AKR_Occlusion.AKR_Occlusion" (* (Math|Conversions|ToFloat(Integer) (Utilities|Array|Length _outhits)) (Variables|Default|GetOcclusionPercentage)) 1000)
        (Development|PrintString (Utilities|String|ToString(Float) (* (Math|Conversions|ToFloat(Integer) (Utilities|Array|Length _outhits)) (Variables|Default|GetOcclusionPercentage))))
        (else
          (Development|PrintString "ISN'T_Occluded" true true "(R=0.000000,G=0.660000,B=1.000000,A=1.000000)" 2.0 "dfgdfhdfh")
          (Class|AkGameplayStatics|SetRTPCValue "/Game/WwiseAudio/Game_Parameters/Default_Work_Unit/Ambience/AKR_Occlusion.AKR_Occlusion" 0.0 1000))))))