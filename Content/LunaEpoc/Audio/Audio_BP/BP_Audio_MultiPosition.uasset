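; Wwise ambience actor that plays looping wind at windows and industrial fan sound at vents.
; On BeginPlay it gathers the transforms of all BP_ArchKit_Window and BP_Audio_Vent actors into separate arrays.
; Each array feeds SetMultiplePositions in MultiSources mode before its loop event is posted.
; Both passes use the same AkDebug component, so the vent positions are set after, and over, the window ones.
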(event EventBeginPlay
  (Utilities|FlowControl|Sequence
    (:then_0
      (bind _outactors (Actor|GetAllActorsOfClass "/Game/LunaEpoc/Assets/Architecture/BP_ArchKit_Window.BP_ArchKit_Window_C"))
      (for _array_element _outactors
        (Utilities|Array|Add (Variables|Default|GetTransform%20Array_Windows) (Transformation|GetActorTransform _array_element)))
      (Class|AkGameplayStatics|SetMultiplePositions (Variables|Default|GetAk%20Debug) (Variables|Default|GetTransform%20Array_Windows) "MultiSources")
      (Class|AkGameObject|PostAkEvent (Variables|Default|GetAk%20Debug) "/Game/LunaEpoc/Audio/Events/Default_Work_Unit/Ambience/Environments/AKE_PlayAmb_Wind_Lp.AKE_PlayAmb_Wind_Lp"))
    (:then_1
      (bind _outactors_2 (Actor|GetAllActorsOfClass "/Game/LunaEpoc/Audio/Audio_BP/BP_Audio_Vent.BP_Audio_Vent_C"))
      (for _array_element_2 _outactors_2
        (Utilities|Array|Add (Variables|Default|GetTransformArray_Vent) (Transformation|GetActorTransform _array_element_2)))
      (Class|AkGameplayStatics|SetMultiplePositions (Variables|Default|GetAk%20Debug) (Variables|Default|GetTransformArray_Vent) "MultiSources")
      (Class|AkGameObject|PostAkEvent (Variables|Default|GetAk%20Debug) "/Game/LunaEpoc/Audio/Events/Default_Work_Unit/Ambience/Environments/AKE_PlayAmb_IndustrialFan_Lp.AKE_PlayAmb_IndustrialFan_Lp"))))

(fn ConstructionScript)