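; Test AI Blueprint that tracks the player through AI perception and feeds the result to the Blackboard.
; Sensing a Player-tagged actor cancels the lose-sight timer and sets CanSeeTarget and TargetActor.
; Any other perception update starts a LineOfSightTimer-length timer that clears both keys on expiry, giving a grace period before the target is forgotten.
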(event OnTargetPerceptionUpdated(AIPerception)
  (params (Actor :type Actor%20Object%20Reference) (Stimulus :type AI%20Stimulus%20Structure))
  (bind _returnvalue (AI|GetBlackboard 0))
  (if (and (Actor|ActorHasTag Actor "Player") (.bSuccessfullySensed (Utilities|Struct|BreakAIStimulus Stimulus)))
    (Utilities|Time|ClearandInvalidateTimerbyHandle (Variables|Default|GetEnemyTimer))
    (AI|Components|Blackboard|SetValueasBool _returnvalue (Variables|Default|GetCanSeeTarget) true)
    (AI|Components|Blackboard|SetValueasObject _returnvalue (Variables|Default|GetTargetActor) Actor)
    (else
      (bind _returnvalue_2 (Utilities|Time|SetTimerbyEvent (delegate Custom|StartEnemyTimer) (Variables|Default|GetLineOfSightTimer)))
      (Variables|Default|SetEnemyTimer _returnvalue_2))))

(event Custom|StartEnemyTimer
  (bind _returnvalue (AI|GetBlackboard 0))
  (AI|Components|Blackboard|SetValueasBool _returnvalue (Variables|Default|GetCanSeeTarget) false)
  (AI|Components|Blackboard|SetValueasObject _returnvalue (Variables|Default|GetTargetActor) 0))

(event EventBeginPlay)

(event Collision|EventActorBeginOverlap
  (params (OtherActor :type Actor%20Object%20Reference)))

(event EventTick
  (params (DeltaSeconds :type Float%20%28single-precision%29)))

(fn ConstructionScript)